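; BP_BigButton is an element-themed weight button that reacts visually when its WeightButton component changes triggered state.
; The construction script takes color, element and particle effect from ElementData, passing the element to WeightButton and creating a dynamic material on the cube.
; At runtime, the trigger-changed event swaps the color parameter between triggered and normal colors, toggles the particles and teleports the cube slightly down or back to rest.
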(event `self.ReceiveBeginPlay`
  (add `WeightButtonComponent.OnButtonTriggeredChanged` (`self.WeightButton`) (delegate `OnChange`)))

(event `OnChange`
  (bind _matrialinst (`self.MatrialInst`))
  (bind _particleeffect (`self.ParticleEffect`))
  (bind _cube (`self.Cube`))
  (bind _colorparameter_name (`self.ColorParameter Name`))
  (if (`WeightButtonComponent.IsTriggered` (`self.WeightButton`))
    (`MaterialInstanceDynamic.SetVectorParameterValue` _matrialinst _colorparameter_name (`KismetMathLibrary.Conv_ColorToLinearColor` (`self.TriggredColor`)))
    (`ActorComponent.SetActive` _particleeffect true false)
    (`SceneComponent.K2_SetRelativeLocation` _cube (0.0 0.0 -5.0) false true)
    (else
      (`MaterialInstanceDynamic.SetVectorParameterValue` _matrialinst _colorparameter_name (`KismetMathLibrary.Conv_ColorToLinearColor` (`self.NormalColor`)))
      (`ActorComponent.SetActive` _particleeffect false false)
      (`SceneComponent.K2_SetRelativeLocation` _cube (0.0 0.0 0.0) false true))))

(fn `UserConstructionScript`
  (bind _elementdata (`self.ElementData`))
  (set `self.NormalColor` (`/Game/Project/Data/Elemental/ElementalData.Color` _elementdata))
  (set `WeightButtonComponent.Element` (`/Game/Project/Data/Elemental/ElementalData.Element` _elementdata) (`self.WeightButton`))
  (`ParticleSystemComponent.SetTemplate` (`self.ParticleEffect`) (`/Game/Project/Data/Elemental/ElementalData.Effects` _elementdata))
  (bind _returnvalue (`PrimitiveComponent.CreateDynamicMaterialInstance` (`self.Cube`) 0 "/Game/Project/Materials/MM_DefaultColor.MM_DefaultColor" "None"))
  (bind _output_get (set `self.MatrialInst` _returnvalue))
  (`MaterialInstanceDynamic.SetVectorParameterValue` _output_get (`self.ColorParameter Name`) (`KismetMathLibrary.Conv_ColorToLinearColor` (`self.NormalColor`))))