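; BP_BigChamferCube is an interactable cube that carries an element and snaps back to its starting transform when its box overlaps a tagged actor.
; The construction script passes the element to its ButtonTrigger and tints a dynamic material with the element color.
; On overlap, it has the player character free the cube, then teleports it to the transform saved at BeginPlay and zeroes linear velocity.
; InteractPreview supplies its preview text.
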(event `self.ReceiveBeginPlay`
  ;[1 1 1] Begin
  (set `self.StartTransform` (`self.GetTransform`)))

(event `self.Box.OnComponentBeginOverlap`
  (params (OverlappedComponent :type "PrimitiveComponent Object Reference") (OtherActor :type "Actor Object Reference") (OtherComp :type "PrimitiveComponent Object Reference") (OtherBodyIndex :type Integer) (bFromSweep :type Boolean) (SweepResult :type "HitResult Structure (by ref)"))
  ;[1 1 1] OnOverlap
  (if (`self.ActorHasTag` OtherActor (`self.Tag`))
    (`|ExecutionSequence`
      (:`then_0`
        (bind _asbp_custom_first_pcharacter (cast `/Game/Project/BluePrints/BP_CustomFirstPCharacter` (`GameplayStatics.GetPlayerPawn` 0)))
        (`/Game/Project/BluePrints/BP_CustomFirstPCharacter.FreeCube` _asbp_custom_first_pcharacter self))
      (:`then_1`
        (`self.ResetTransform`)))))

(fn `InteractPreview`
  (returns (previewText :type Text))
  (return (`self.PreviewText`)))

(fn `ResetTransform`
  (`self.K2_SetActorTransform` (`self.StartTransform`) false true)
  (`PrimitiveComponent.SetAllPhysicsLinearVelocity` (`self.StaticMeshComponent`) (0.0 0.0 0.0) false))

(fn `UserConstructionScript`
  (bind _elemtdata (`self.ElemtData`))
  (set `self.Normal Color` (`/Game/Project/Data/Elemental/ElementalData.Color` _elemtdata))
  (set `ButtonTriggerComponent.Element` (`/Game/Project/Data/Elemental/ElementalData.Element` _elemtdata) (`self.ButtonTrigger`))
  (bind _returnvalue (`PrimitiveComponent.CreateDynamicMaterialInstance` (`self.StaticMeshComponent`) 0 "/Game/Project/Materials/MM_DefaultColor.MM_DefaultColor" "None"))
  (bind _output_get (set `self.Matrial Inst` _returnvalue))
  (`MaterialInstanceDynamic.SetVectorParameterValue` _output_get (`self.ColorParameter Name`) (`KismetMathLibrary.Conv_ColorToLinearColor` (`self.Normal Color`))))